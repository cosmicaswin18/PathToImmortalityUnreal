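; BP_Animal is a hostile roaming animal AI with a camera-facing health bar widget.
; It loops AIMoveTo to random nearby points until PawnSensing sees a Player-tagged pawn, then moves to the player and attacks.
; The attack montage's notify triggers a forward sphere trace that applies damage.
; Incoming damage updates the bar; at zero health it increments the player's KillCount, destroys itself and calls the player's IncreaseHealth.
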(event `self.ReceiveBeginPlay`
  (`self.RoamAround`)
  (bind _output_get (set `self.CurrentHealth` (`self.MaxHealth`)))
  (bind _aswp_enemy_ai_health_bar (cast `/Game/UI/WP_EnemyAI_HealthBar` (`WidgetComponent.GetUserWidgetObject` (`self.Widget`))))
  (`/Game/UI/WP_EnemyAI_HealthBar.Update Health UI` _aswp_enemy_ai_health_bar _output_get (`self.MaxHealth`)))

(event `self.ReceiveTick`
  (params (DeltaSeconds :type "Float (single-precision)"))
  (`SceneComponent.K2_SetWorldRotation` (`self.Widget`) (`KismetMathLibrary.FindLookAtRotation` (`SceneComponent.K2_GetComponentLocation` (`self.Widget`)) (`SceneComponent.K2_GetComponentLocation` (`PlayerCameraManager.TransformComponent` (`GameplayStatics.GetPlayerCameraManager` 0)))) false false))

(event `RoamAround`
  (`|AIMoveTo` self (`NavigationSystemV1.K2_GetRandomReachablePointInRadius` (`self.K2_GetActorLocation`) 1000.0 null null) null 200.0
    (:`OnSuccess`
      (`KismetSystemLibrary.Delay` 3.0)
      (`self.RoamAround`))))

(event `self.PawnSensing.OnSeePawn`
  (params (Pawn :type "Pawn Object Reference"))
  (bind _returnvalue (`self.K2_GetActorLocation`))
  (if (`self.ActorHasTag` Pawn "Player")
    (`|AIMoveTo` self (0.0 0.0 0.0) (`GameplayStatics.GetPlayerCharacter` 0) 200.0
      (:`OnSuccess`
        (if (not (`self.IsAttacking`))
          (set `self.IsAttacking` true)
          (`|PlayMontage` (`self.Mesh`) (`self.AttackMontage`)
            (:`then`
              (`GameplayStatics.PlaySoundAtLocation` "/Game/Audio/Whoosh_Punch3.Whoosh_Punch3" (`self.K2_GetActorLocation`) (struct) 1.0 1.0 0.0 null null null null))
            (:`OnCompleted`
              (set `self.IsAttacking` false))
            (:`OnNotifyBegin`
              (bind (_outhit _returnvalue_2) (`KismetSystemLibrary.SphereTraceSingleForObjects` _returnvalue (+ _returnvalue (* (`KismetMathLibrary.GetForwardVector` (`self.K2_GetActorRotation`)) 300.0)) 100.0 (`|MakeArray` "ObjectTypeQuery3" :!type "EObjectTypeQuery Enum")))
              (if _returnvalue_2
                (`GameplayStatics.ApplyDamage` (`.HitActor` (`GameplayStatics.BreakHitResult` _outhit)) (`self.AttackDamage`))))))))))

(event `self.ReceiveAnyDamage`
  (params (Damage :type "Float (single-precision)") (DamageType :type "DamageType Object Reference") (InstigatedBy :type "Controller Object Reference") (DamageCauser :type "Actor Object Reference"))
  (bind _output_get (set `self.CurrentHealth` (- (`self.CurrentHealth`) Damage)))
  (bind _aswp_enemy_ai_health_bar (cast `/Game/UI/WP_EnemyAI_HealthBar` (`WidgetComponent.GetUserWidgetObject` (`self.Widget`))))
  (`/Game/UI/WP_EnemyAI_HealthBar.Update Health UI` _aswp_enemy_ai_health_bar _output_get (`self.MaxHealth`))
  (if (<= (`self.CurrentHealth`) 0.0)
    (`|ExecutionSequence`
      (:`then_0`
        (bind _asbp_third_person_character (cast `/Game/ThirdPerson/Blueprints/BP_ThirdPersonCharacter` (`GameplayStatics.GetPlayerCharacter` 0)))
        (`/Engine/EditorBlueprintResources/StandardMacros.IncrementInt` (`/Game/ThirdPerson/Blueprints/BP_ThirdPersonCharacter.KillCount` _asbp_third_person_character)))
      (:`then_1`
        (`self.K2_DestroyActor`))
      (:`then_2`
        (`/Game/ThirdPerson/Blueprints/BP_ThirdPersonCharacter.IncreaseHealth` _asbp_third_person_character)))))

(fn `UserConstructionScript`)